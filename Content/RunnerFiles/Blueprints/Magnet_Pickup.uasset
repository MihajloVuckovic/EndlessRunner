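; Magnet power-up pickup for the runner that switches on the ThirdPersonCharacter's magnet for a timed period.
; On overlap it plays a sound, hides its mesh, stores duration and pickup time on the character, and starts a one-shot timer.
; When the timer fires, it clears the magnet flag and destroys itself only if time since the character's latest pickup exceeds the duration.
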(event Custom|onTimerExpiration
  (bind _asthird_person_character (Utilities|Casting|CastToThirdPersonCharacter (Game|GetPlayerCharacter 0)))
  (if (Variables|/Game/ThirdPersonBP/Blueprints/ThirdPersonCharacter.ThirdPersonCharacter_C|GetMagnetActive _asthird_person_character)
    (Variables|/Game/ThirdPersonBP/Blueprints/ThirdPersonCharacter.ThirdPersonCharacter_C|SetMagnetActive _asthird_person_character false)
    (Actor|DestroyActor)))

(event Custom|Timer
  (bind _asthird_person_character (Utilities|Casting|CastToThirdPersonCharacter (Game|GetPlayerCharacter 0)))
  (if (Variables|/Game/ThirdPersonBP/Blueprints/ThirdPersonCharacter.ThirdPersonCharacter_C|GetMagnetActive _asthird_person_character)
    (bind _output_get (Variables|/Game/ThirdPersonBP/Blueprints/ThirdPersonCharacter.ThirdPersonCharacter_C|SetMagnetElapsedTime _asthird_person_character (- (Utilities|Time|GetGameTimeinSeconds) (Variables|/Game/ThirdPersonBP/Blueprints/ThirdPersonCharacter.ThirdPersonCharacter_C|GetMagnetPickupTime _asthird_person_character))))
    (if (< (- (Variables|/Game/ThirdPersonBP/Blueprints/ThirdPersonCharacter.ThirdPersonCharacter_C|GetMagnetTimer _asthird_person_character) _output_get) 0.0)
      (CallFunction|OnTimerExpiration))))

(event Collision|EventActorBeginOverlap
  (params (OtherActor :type Actor%20Object%20Reference))
  (bind _asthird_person_character (Utilities|Casting|CastToThirdPersonCharacter OtherActor))
  (Variables|/Game/ThirdPersonBP/Blueprints/ThirdPersonCharacter.ThirdPersonCharacter_C|SetMagnetActive _asthird_person_character true)
  (Audio|PlaySound2D "/Game/RunnerFiles/SFX/Laser_Pull.Laser_Pull" 1.0 1.0 0.0 0 0)
  (Rendering|SetVisibility (Variables|Default|GetStaticMesh) false false)
  (bind _output_get (Variables|/Game/ThirdPersonBP/Blueprints/ThirdPersonCharacter.ThirdPersonCharacter_C|SetMagnetTimer _asthird_person_character 1e+01))
  (Variables|/Game/ThirdPersonBP/Blueprints/ThirdPersonCharacter.ThirdPersonCharacter_C|SetMagnetPickupTime _asthird_person_character (Utilities|Time|GetGameTimeinSeconds))
  (if (Variables|/Game/ThirdPersonBP/Blueprints/ThirdPersonCharacter.ThirdPersonCharacter_C|GetMagnetActive _asthird_person_character)
    (Utilities|Time|SetTimerbyEvent (delegate Custom|Timer) _output_get)))

(fn ConstructionScript)