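; Boots pickup that gives the ThirdPersonCharacter a timed jump boost on overlap.
; Overlap sets the boots state, duration and pickup time on the character, raises JumpZVelocity, plays a sound and hides the mesh, leaving collision untouched.
; A one-shot timer then compares elapsed time to the duration on player 0's character.
; Only if strictly exceeded does it restore jump velocity, clear the active flag and destroy the pickup.
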(event Custom|Timer
  (bind _asthird_person_character (Utilities|Casting|CastToThirdPersonCharacter (Game|GetPlayerCharacter 0)))
  (bind _output_get (Variables|/Game/ThirdPersonBP/Blueprints/ThirdPersonCharacter.ThirdPersonCharacter_C|SetBootsElapsedTime _asthird_person_character (- (Utilities|Time|GetGameTimeinSeconds) (Variables|/Game/ThirdPersonBP/Blueprints/ThirdPersonCharacter.ThirdPersonCharacter_C|GetBootsPickupTime _asthird_person_character))))
  (if (< (- (Variables|/Game/ThirdPersonBP/Blueprints/ThirdPersonCharacter.ThirdPersonCharacter_C|GetBootsTimer _asthird_person_character) _output_get) 0.0)
    (CallFunction|TimerExpired)))

(event Custom|TimerExpired
  (bind _asthird_person_character (Utilities|Casting|CastToThirdPersonCharacter (Game|GetPlayerCharacter 0)))
  (Variables|/Script/Engine.CharacterMovementComponent|SetJumpZVelocity (Variables|/Script/Engine.Character|GetCharacterMovement _asthird_person_character) 6e+02)
  (Variables|/Game/ThirdPersonBP/Blueprints/ThirdPersonCharacter.ThirdPersonCharacter_C|SetBootsActive _asthird_person_character false)
  (Actor|DestroyActor))

(event EventBeginPlay)

(event Collision|EventActorBeginOverlap
  (params (OtherActor :type Actor%20Object%20Reference))
  (bind _asthird_person_character (Utilities|Casting|CastToThirdPersonCharacter OtherActor))
  (Variables|/Game/ThirdPersonBP/Blueprints/ThirdPersonCharacter.ThirdPersonCharacter_C|SetBootsActive _asthird_person_character true)
  (Audio|PlaySound2D "/Game/RunnerFiles/SFX/Object_PickUp.Object_PickUp" 1.0 1.0 0.0 0 0)
  (Variables|/Script/Engine.CharacterMovementComponent|SetJumpZVelocity (Variables|/Script/Engine.Character|GetCharacterMovement _asthird_person_character) 8e+02)
  (Rendering|SetVisibility (Variables|Default|GetStaticMesh) false false)
  (bind _output_get (Variables|/Game/ThirdPersonBP/Blueprints/ThirdPersonCharacter.ThirdPersonCharacter_C|SetBootsTimer _asthird_person_character 1e+01))
  (Variables|/Game/ThirdPersonBP/Blueprints/ThirdPersonCharacter.ThirdPersonCharacter_C|SetBootsPickupTime _asthird_person_character (Utilities|Time|GetGameTimeinSeconds))
  (Utilities|Time|SetTimerbyEvent (delegate Custom|Timer) _output_get))

(fn ConstructionScript)